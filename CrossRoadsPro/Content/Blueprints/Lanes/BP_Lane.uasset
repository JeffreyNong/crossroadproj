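; BP_Lane is one lane in an endless road-crossing game, with moving cars and randomly scattered decor.
; Tick uses a Delay to spawn random cars at random intervals, and an end-of-lane trigger destroys them.
; The player's first overlap adds score and asks LaneSpawner for another lane.
; BeginPlay places decor along Y using distance-weighted odds, while ReverseLane mirrors spawn point, exit trigger and speed to flip traffic.
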(event OnComponentBeginOverlap(PlayerTriggerZone)
  (params (OverlappedComponent :type Primitive%20Component%20Object%20Reference) (OtherActor :type Actor%20Object%20Reference) (OtherComp :type Primitive%20Component%20Object%20Reference) (OtherBodyIndex :type Integer) (bFromSweep :type Boolean) (SweepResult :type Hit%20Result%20Structure%20%28by%20ref%29))
  (bind _asbp_player (Utilities|Casting|CastToBP_Player OtherActor))
  (if (not (Variables|Default|GetTraveled))
    (Default|SpawnLaneatSpawnPoint (Variables|Default|GetLaneSpawner))
    (Default|AddScore _asbp_player 1)
    (Variables|Default|SetTraveled true)))

(event OnComponentEndOverlap(CarTriggerZone)
  (params (OverlappedComponent :type Primitive%20Component%20Object%20Reference) (OtherActor :type Actor%20Object%20Reference) (OtherComp :type Primitive%20Component%20Object%20Reference) (OtherBodyIndex :type Integer))
  (bind _asbp_car (Utilities|Casting|CastToBP_Car OtherActor))
  (Utilities|Array|RemoveItem (Variables|Default|GetCars) _asbp_car)
  (Actor|DestroyActor _asbp_car))

(event EventBeginPlay
  (CallFunction|GenerateDecor))

(event EventTick
  (params (DeltaSeconds :type Float%20%28single-precision%29))
  (if (Utilities|Array|IsValidIndex (Variables|Default|GetCarTypes))
    (Utilities|FlowControl|Delay (Math|Random|RandomFloatinRange (Variables|Default|GetMinSpawnTime) (Variables|Default|GetMaxSpawnTime)))
    (CallFunction|SpawnCar)))

(fn ConstructionScript)

(fn SpawnCar
  (bind _returnvalue (Game|SpawnActorfromClass (.OutItem (Utilities|Array|Random (Variables|Default|GetCarTypes))) (Math|Transform|MakeTransform (Transformation|GetWorldLocation (Variables|Default|GetCarSpawnPoint)) "0, 0, 0" "1,1,1") "Undefined" 0 0))
  (Variables|/Game/Blueprints/Cars/BP_Car.BP_Car_C|Setspeed _returnvalue (Variables|Default|GetVehicleSpeed))
  (Utilities|Array|Add (Variables|Default|GetCars) _returnvalue))

(fn DestroyLane
  (for _array_element (Variables|Default|GetCars)
    (Actor|DestroyActor _array_element))
  (Actor|DestroyActor))

(fn ReverseLane
  (bind _cartriggerzone (Variables|Default|GetCarTriggerZone))
  (bind _carspawnpoint (Variables|Default|GetCarSpawnPoint))
  (Transformation|SetRelativeLocation _cartriggerzone (Math|Vector|MakeVector 0.0 (* -1 (.y (Variables|/Script/Engine.SceneComponent|GetRelativeLocation _cartriggerzone))) 0.0) false false)
  (Transformation|SetRelativeLocation _carspawnpoint (Math|Vector|MakeVector 0.0 (* -1 (.y (Variables|/Script/Engine.SceneComponent|GetRelativeLocation _carspawnpoint))) 0.0) false false)
  (Variables|Default|SetVehicleSpeed (* -1 (Variables|Default|GetVehicleSpeed))))

(fn GenerateDecor
  (bind _self self)
  (bind _returnvalue (Transformation|GetActorLocation _self))
  (if (> (Utilities|Array|Length (Variables|Default|GetDecorTypes)) 0)
    (for _index (range -20 20)
      (bind _odds (CallFunction|PickDecorOdds _index))
      (if (<= (Math|Random|RandomFloat) _odds)
        (Game|SpawnActorfromClass (.OutItem (Utilities|Array|Random (Variables|Default|GetDecorTypes))) (Math|Transform|MakeTransform (Math|Vector|MakeVector (.x _returnvalue) (+ (* _index 8e+01) (.y _returnvalue)) (.z _returnvalue)) "0, 0, 0" "1,1,1") "Undefined" 0 0)))))

(fn PickDecorOdds
  (params (DistanceInt :type Integer))
  (bind _keys (Utilities|Map|Keys (Variables|Default|GetDecorWeighting)))
  (for (_array_element _array_index) _keys
    (if (>= (Math|Integer|Absolute(Integer) DistanceInt) _array_element)
      (bind _values (Utilities|Map|Values (Variables|Default|GetDecorWeighting)))
      (return (Utilities|Array|Get(acopy) _values _array_index))))
  (return 0.0))